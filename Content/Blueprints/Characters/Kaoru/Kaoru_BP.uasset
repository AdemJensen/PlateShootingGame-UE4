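; Kaoru character Blueprint that takes damage, reacts with voice and animation, and dies into a ragdoll.
; AnyDamage subtracts Health, and a lethal hit awards score to the instigator's MyPlayerState before calling Die, which only runs if that cast succeeds.
; HurtSounds plays a damage animation and a heavy or randomly chosen light voice cue, gated by a short cooldown.
; DieOnServer is empty, and the SlowHealthBar widget logic is disconnected.
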(event Custom|Die
  (params (Instigator :type Controller%20Object%20Reference))
  (bind _mesh (Variables|Character|GetMesh))
  (bind _mesh_2 (Variables|Character|GetMesh))
  (bind _mesh_3 (Variables|Character|GetMesh))
  (Collision|SetCollisionEnabled (Variables|Collision|GetCapsuleComponent) "NoCollision")
  (Class|SkeletalMeshComponent|SetAllBodiesSimulatePhysics _mesh_2 true)
  (Class|SkeletalMeshComponent|SetAllBodiesPhysicsBlendWeight _mesh_2 1.0 false)
  (Collision|SetCollisionResponsetoChannel _mesh_2 "ECC_Visibility" "ECR_Ignore")
  (Collision|SetCollisionResponsetoChannel _mesh "ECC_PhysicsBody" "ECR_Ignore")
  (Collision|SetCollisionResponsetoChannel _mesh "ECC_Pawn" "ECR_Ignore")
  (Physics|SetSimulatePhysics _mesh_3 true)
  (Physics|SetEnableGravity _mesh_3 true)
  (Audio|PlaySoundatLocation "/Game/Blueprints/Characters/Kaoru/Kaoru_Die_Cue.Kaoru_Die_Cue" (Transformation|GetWorldLocation (Variables|Collision|GetCapsuleComponent)) "0, 0, 0" 1.0 1.0 0.0 0 0 0)
  (Variables|Default|SetisDead true))

(event Custom|Hurt%20Sounds
  (params (Damage :type Float%20%28single-precision%29))
  (if (Variables|Default|GetCan%20Generate%20Hurt%20Voice)
    (Components|Animation|PlayAnimation (Variables|Character|GetMesh) "/Game/ArtMaterials/Kaoru/Animations/Anim_Damage.Anim_Damage" false)
    (if (> Damage 75.0)
      (Audio|PlaySoundatLocation "/Game/Blueprints/Characters/Kaoru/Kaoru_Hurt_Heavy_Cue.Kaoru_Hurt_Heavy_Cue" (Transformation|GetWorldLocation (Variables|Collision|GetCapsuleComponent)) "0, 0, 0" 1.0 1.0 0.0 0 0 0)
      (Variables|Default|SetCan%20Generate%20Hurt%20Voice false :!label _label)
      (Utilities|FlowControl|Delay 0.5)
      (Variables|Default|SetCan%20Generate%20Hurt%20Voice true)
      (elif (> (Math|Random|RandomFloatinRange 0.0 1.0) 0.3)
        (Audio|PlaySoundatLocation "/Game/Blueprints/Characters/Kaoru/Kaoru_Hurt_Light_Cue.Kaoru_Hurt_Light_Cue" (Transformation|GetWorldLocation (Variables|Collision|GetCapsuleComponent)) "0, 0, 0" 1.0 1.0 0.0 0 0 0)
        (goto _label)))))

(event Custom|Die%20On%20Server
  (params (Instigator :type Controller%20Object%20Reference)))

(event EventBeginPlay)

(event Collision|EventActorBeginOverlap
  (params (OtherActor :type Actor%20Object%20Reference)))

(event EventTick
  (params (DeltaSeconds :type Float%20%28single-precision%29)))

(event Game|Damage|EventAnyDamage
  (params (Damage :type Float%20%28single-precision%29) (DamageType :type Damage%20Type%20Object%20Reference) (InstigatedBy :type Controller%20Object%20Reference) (DamageCauser :type Actor%20Object%20Reference))
  (if (not (Variables|Default|GetisDead))
    (bind _output_get (Variables|Default|SetHealth (- (Variables|Default|GetHealth) Damage)))
    (if (<= _output_get 0.0)
      (bind _asmy_player_state (Utilities|Casting|CastToMyPlayerState (Variables|/Script/Engine.Controller|GetPlayerState InstigatedBy)))
      (Default|IncrementScore _asmy_player_state 25)
      (CallFunction|Die InstigatedBy)
      (else
        (CallFunction|HurtSounds Damage)))))

(fn ConstructionScript)