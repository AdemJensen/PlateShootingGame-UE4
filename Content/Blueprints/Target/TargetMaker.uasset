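; TargetMaker is a server-side spawner that keeps creating Target_BP actors at random points within a sphere around itself.
; Tick accumulates time and, past SpawnInterval, spawns when enabled and under MaxTargets, with a negative limit meaning unlimited.
; MakeTarget picks a type index by ratio weights, redrawing the random threshold at each comparison.
; Per-type settings supply scale, health, score, color, movement timing and velocity to the new target.
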(event EventBeginPlay)

(event Collision|EventActorBeginOverlap
  (params (OtherActor :type Actor%20Object%20Reference)))

(event EventTick
  (params (DeltaSeconds :type Float%20%28single-precision%29))
  (if (> (Variables|Default|GetNowTime) (Variables|Settings|GetSpawnInterval))
    (bind _returnvalue (Utilities|ShouldMakeTarget))
    (if _returnvalue
      (Utilities|MakeTarget
        (:Exec
          (Variables|Default|SetNowTime 0.0))))
    (else
      (Variables|Default|SetNowTime (+ DeltaSeconds (Variables|Default|GetNowTime))))))

(fn ConstructionScript)

(fn Sum
  (params (Array :type Array%20of%20Floats%20%28single-precision%29))
  (LocalVariables|SetSummary 0.0)
  (for _array_element Array
    (bind _output_get (LocalVariables|SetSummary (+ _array_element (LocalVariables|GetSummary)))))
  (return _output_get))

(fn RandomChoosebyRatio
  (params (RatioArray :type Array%20of%20Floats%20%28single-precision%29))
  (bind _sum (CallFunction|Sum RatioArray))
  (LocalVariables|SetCurrentAdd 0.0)
  (LocalVariables|SetCurrentIndex 0)
  (for _array_element RatioArray
    (bind _output_get (LocalVariables|SetCurrentAdd (+ (LocalVariables|GetCurrentAdd) _array_element)))
    (if (>= _output_get (Math|Random|RandomFloatinRange 0.0 _sum))
      (return (LocalVariables|GetCurrentIndex))
      (else
        (Math|Integer|IncrementInt (LocalVariables|GetCurrentIndex)))))
  (return (- (Utilities|Array|Length RatioArray) 1)))