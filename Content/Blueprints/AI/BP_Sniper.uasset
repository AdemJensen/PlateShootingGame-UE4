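; BP_Sniper is an AI bot character that starts the game armed with an AW50 weapon.
; On BeginPlay the server spawns the AW50, marks it as not needing reload, adds and equips it through PickupFunctionModule, and gives the player state a generated "BOT_" nickname.
; Taking damage runs the parent handling, then sets the blackboard's retreat flag so the AI can react to being hit.
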(event EventBeginPlay
  (if (Networking|IsServer)
    (bind _returnvalue (Game|SpawnActorfromClass "/Game/Blueprints/Weapons/AW-50.AW-50_C" (Transformation|GetWorldTransform (Variables|Character|GetMesh)) "AlwaysSpawn" 0 0))
    (bind _output_get (Variables|Default|SetPreset%20Weapon _returnvalue))
    (Variables|/Script/PlateShootingGame.Weapon|SetbNeedsReload _output_get false)
    (Class|PickupFunctionModule|AddItemtoList (Variables|Default|GetPickupFunctionModule) (Variables|Default|GetPreset%20Weapon))
    (Class|PickupFunctionModule|PickupItem (Variables|Default|GetPickupFunctionModule) (Variables|Default|GetPreset%20Weapon))
    (bind _asmy_player_state (Utilities|Casting|CastToMyPlayerState (Variables|Default|GetPlayerState)))
    (Variables|/Game/Blueprints/MyPlayerState.MyPlayerState_C|SetPlayerNickname _asmy_player_state (Utilities|String|Append "BOT_" (Class|DataGeneratorLib|GenerateUsername)))))

(event Collision|EventActorBeginOverlap
  (params (OtherActor :type Actor%20Object%20Reference)))

(event EventTick
  (params (DeltaSeconds :type Float%20%28single-precision%29)))

(event EventTakeDamageBP
  (params (DamageAmount :type Float%20%28single-precision%29) (EventInstigator :type Pawn%20Object%20Reference) (DamageCauser :type Actor%20Object%20Reference))
  (|CallParentFunction DamageAmount EventInstigator DamageCauser)
  (AI|Components|Blackboard|SetValueasBool (AI|GetBlackboard self) (Variables|Default|GetBBK_NeedsRetreat) true))

(fn ConstructionScript)