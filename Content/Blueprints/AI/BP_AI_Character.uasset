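; AI-controlled bot character for a shooter, spawning on the server with an AR15 and a generated BOT_ nickname.
; Perception and damage events choose a sighted enemy, cleared on its death or re-evaluated by delayed timers, and write it to the Blackboard with retreat and death flags.
; Shots aim at that enemy with random rotational spread.
; Death updates killer and victim scores, then requests a delayed respawn from the game mode.
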(event OnTargetPerceptionUpdated(AIPerception)
  (params (Actor :type Actor%20Object%20Reference) (Stimulus :type AI%20Stimulus%20Structure))
  (if (and (not (Variables|Default|GetbDead)) (Networking|IsServer))
    (Utilities|IsValid Actor
      (:Is%20Valid
        (bind _asshooter_game_character_base (Utilities|Casting|CastToShooterGameCharacterBase Actor))
        (if (and (.bSuccessfullySensed (Utilities|Struct|BreakAIStimulus Stimulus)) (or (Actor|ActorHasTag Actor "PlayerControlledCharacter") (not (Variables|Default|GetScan%20Human%20Player%20Only))))
          (if (not (Variables|/Script/PlateShootingGame.ShooterGameCharacterBase|GetbDead _asshooter_game_character_base))
            (Utilities|Array|AddUnique (Variables|Default|GetSighted%20Enemies) _asshooter_game_character_base)
            (Utilities|IsValid (Variables|Default|GetSighted%20Enemy)
              (:Is%20Not%20Valid
                (bind _output_get (Variables|Default|SetSighted%20Enemy _asshooter_game_character_base))
                (AI|Components|Blackboard|SetValueasObject (AI|GetBlackboard self) (Variables|Default|GetBBK_Sighted%20Enemy) _output_get))))
          (else
            (bind _returnvalue (Utilities|Array|RemoveItem (Variables|Default|GetSighted%20Enemies) _asshooter_game_character_base))
            (if _returnvalue
              (bind _returnvalue_2 (Utilities|Time|SetTimerbyEvent (delegate Custom|Reset%20Sight) 5.0))
              (Variables|Default|SetSight%20Timer _returnvalue_2))))))))

(event Custom|Reset%20Sight
  (bind _sighted_enemies (Variables|Default|GetSighted%20Enemies))
  (if (and (not (Utilities|Array|ContainsItem (Variables|Default|GetSighted%20Enemies) (stale OnTargetPerceptionUpdated(AIPerception) _asshooter_game_character_base))) (== (stale OnTargetPerceptionUpdated(AIPerception) _asshooter_game_character_base) (Variables|Default|GetSighted%20Enemy)))
    (bind _output_get (Variables|Default|SetSighted%20Enemy (select (Utilities|Array|IsValidIndex _sighted_enemies) (Utilities|Array|Get(acopy) _sighted_enemies) 0)))
    (AI|Components|Blackboard|SetValueasObject (AI|GetBlackboard self) (Variables|Default|GetBBK_Sighted%20Enemy) _output_get)))

(event EventBeginPlay
  (if (Networking|IsServer)
    (bind _returnvalue (Game|SpawnActorfromClass "/Game/Blueprints/Weapons/AR-15.AR-15_C" (Transformation|GetWorldTransform (Variables|Character|GetMesh)) "AlwaysSpawn" 0 0))
    (bind _output_get (Variables|Default|SetPreset%20Weapon _returnvalue))
    (Variables|/Script/PlateShootingGame.Weapon|SetbNeedsReload _output_get false)
    (Class|PickupFunctionModule|AddItemtoList (Variables|Default|GetPickupFunctionModule) (Variables|Default|GetPreset%20Weapon))
    (Class|PickupFunctionModule|PickupItem (Variables|Default|GetPickupFunctionModule) (Variables|Default|GetPreset%20Weapon))
    (bind _asmy_player_state (Utilities|Casting|CastToMyPlayerState (Variables|Default|GetPlayerState)))
    (Variables|/Game/Blueprints/MyPlayerState.MyPlayerState_C|SetPlayerNickname _asmy_player_state (Utilities|String|Append "BOT_" (Class|DataGeneratorLib|GenerateUsername)))))

(event Collision|EventActorBeginOverlap
  (params (OtherActor :type Actor%20Object%20Reference)))

(event EventTick
  (params (DeltaSeconds :type Float%20%28single-precision%29))
  (bind _sighted_enemies (Variables|Default|GetSighted%20Enemies))
  (|CallParentFunction DeltaSeconds)
  (Utilities|FlowControl|Sequence
    (:then_0
      (Utilities|IsValid (Variables|Default|GetSighted%20Enemy)
        (:Is%20Valid
          (if (Variables|/Script/PlateShootingGame.ShooterGameCharacterBase|GetbDead (Variables|Default|GetSighted%20Enemy))
            (Utilities|Time|ClearandInvalidateTimerbyHandle (Variables|Default|GetSight%20Timer))
            (Variables|Default|SetSighted%20Enemy 0)
            (AI|Components|Blackboard|SetValueasObject (AI|GetBlackboard self) (Variables|Default|GetBBK_Sighted%20Enemy) 0)))))
    (:then_1
      (for _array_element _sighted_enemies
        (Utilities|IsValid _array_element
          (:Is%20Valid
            (if (Variables|/Script/PlateShootingGame.ShooterGameCharacterBase|GetbDead _array_element)
              (Utilities|Array|RemoveItem _sighted_enemies _array_element :!label _label)))
          (:Is%20Not%20Valid
            (goto _label)))))))

(event EventAdjustShootingDirection
  (bind _sighted_enemy (Variables|Default|GetSighted%20Enemy))
  (bind _shoot_precision (Variables|Default|GetShoot%20Precision))
  (bind _weaponinhand (Variables|Default|GetWeaponInHand))
  (bind _returnvalue (* _shoot_precision -1.0))
  (Utilities|IsValid (Variables|Default|GetWeaponInHand)
    (:Is%20Valid
      (Utilities|IsValid _sighted_enemy
        (:Is%20Valid
          (bind _returnvalue_2 (Class|Weapon|GetGunPortLocation (Variables|Default|GetWeaponInHand)))
          (Class|Weapon|SetFireDirection (Variables|Default|GetWeaponInHand) (Math|Vector|RotateVector (- (Transformation|GetActorLocation _sighted_enemy) _returnvalue_2) (Math|Rotator|MakeRotator (Math|Random|RandomFloatinRange _returnvalue _shoot_precision) (Math|Random|RandomFloatinRange _returnvalue _shoot_precision) (Math|Random|RandomFloatinRange _returnvalue _shoot_precision)))))
        (:Is%20Not%20Valid
          (bind _returnvalue_3 (Class|Weapon|GetGunPortDirection _weaponinhand))
          (Class|Weapon|SetFireDirection _weaponinhand _returnvalue_3))))))

(event EventActionDieBPonServer
  (params (EventInstigator :type Pawn%20Object%20Reference) (DamageCauser :type Actor%20Object%20Reference))
  (Variables|/Script/PlateShootingGame.Weapon|SetbNeedsReload (Variables|Default|GetPreset%20Weapon) true)
  (AI|Components|Blackboard|SetValueasBool (AI|GetBlackboard self) (Variables|Default|GetBBK_Dead) true)
  (Utilities|IsValid EventInstigator
    (:Is%20Valid
      (bind _asmy_player_state (Utilities|Casting|CastToMyPlayerState (Variables|/Script/Engine.Pawn|GetPlayerState EventInstigator))
        (:then
          (Default|IncrementScore _asmy_player_state 1))
        (:CastFailed
          _)))
    (:Is%20Not%20Valid
      _))
  (bind _asmy_player_state_2 (Utilities|Casting|CastToMyPlayerState (Variables|Default|GetPlayerState))
    (:then
      (Default|IncrementDeath _asmy_player_state_2))
    (:CastFailed
      _))
  (Utilities|FlowControl|Delay 3.0)
  (bind _astemporary_game_mode (Utilities|Casting|CastToTemporaryGameMode (Game|GetGameMode)))
  (bind _asai_controller (Utilities|Casting|CastToAI_Controller (Pawn|GetController)))
  (Default|RespawnAIPlayer _astemporary_game_mode _asai_controller (Utilities|GetClass self)))

(event EventTakeDamageBP
  (params (DamageAmount :type Float%20%28single-precision%29) (EventInstigator :type Pawn%20Object%20Reference) (DamageCauser :type Actor%20Object%20Reference))
  (Utilities|FlowControl|Sequence
    (:then_0
      (bind _asshooter_game_character_base (Utilities|Casting|CastToShooterGameCharacterBase EventInstigator))
      (bind _output_get (Variables|Default|SetSighted%20Enemy _asshooter_game_character_base))
      (AI|Components|Blackboard|SetValueasObject (AI|GetBlackboard self) (Variables|Default|GetBBK_Sighted%20Enemy) _output_get)
      (Utilities|Time|ClearandInvalidateTimerbyHandle (Variables|Default|GetDamage%20Timer))
      (bind _returnvalue (Utilities|Time|SetTimerbyEvent (delegate Custom|Reset%20Sight) 5.0))
      (Variables|Default|SetDamage%20Timer _returnvalue))
    (:then_1
      (AI|Components|Blackboard|SetValueasBool (AI|GetBlackboard self) (Variables|Default|GetBBK_NeedsRetreat) (< (Class|ShooterGameCharacterBase|GetHealthPercentage) 0.3)))))

(fn ConstructionScript
  (|CallParentFunction)
  (Utilities|Array|AddUnique (Variables|Default|GetTags) "AIControlledCharacter"))