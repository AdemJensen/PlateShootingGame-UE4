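; Behavior Tree task that picks a location for an AI pawn to hold an accepted range from its approach target.
; It projects a point at that range from the target along the direction toward the pawn, then finds a random reachable navigation point within a fixed radius around it.
; The point is written to the next target location Blackboard key; the task fails if the target or point is unavailable.
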(event EventReceiveExecuteAI
  (params (OwnerController :type AI%20Controller%20Object%20Reference) (ControlledPawn :type Pawn%20Object%20Reference))
  (bind _asactor (Utilities|Casting|CastToActor (Class|BTFunctionLibrary|GetBlackboardValueasObject (Variables|Default|GetApproach%20Target)))
    (:then
      (if (.ReturnValue (AI|Navigation|GetRandomReachablePointinRadius (+ (* (Math|Vector|Normalize (- (Transformation|GetActorLocation ControlledPawn) (Transformation|GetActorLocation _asactor))) (Variables|Default|GetAccepted%20Range)) (Transformation|GetActorLocation _asactor)) 5e+02 0 0))
        (AI|BehaviorTree|SetBlackboardValueasVector (Variables|Default|GetNext%20Target%20Location) (.RandomLocation (AI|Navigation|GetRandomReachablePointinRadius (+ (* (Math|Vector|Normalize (- (Transformation|GetActorLocation ControlledPawn) (Transformation|GetActorLocation _asactor))) (Variables|Default|GetAccepted%20Range)) (Transformation|GetActorLocation _asactor)) 5e+02 0 0)))
        (AI|BehaviorTree|FinishExecute true)
        (else
          (AI|BehaviorTree|FinishExecute false))))
    (:CastFailed
      (AI|BehaviorTree|FinishExecute false))))