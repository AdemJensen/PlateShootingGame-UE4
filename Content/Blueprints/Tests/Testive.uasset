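; Test pickup actor, apparently an assault rifle ammo pickup, with partly stubbed pickup logic.
; OperationRange overlaps check for I_HoldableCharacter: begin only casts, while end calls an empty OnPickup.
; HandlePickup refills a TestiveCharacter_BP weapon's magazine and plays a reload sound through ClientPlaySound, but its only call in this graph is disconnected.
; IsOpenForPickup always returns false and GetPickableInfo returns nothing.
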(event OnComponentBeginOverlap(OperationRange)
  (params (OverlappedComponent :type Primitive%20Component%20Object%20Reference) (OtherActor :type Actor%20Object%20Reference) (OtherComp :type Primitive%20Component%20Object%20Reference) (OtherBodyIndex :type Integer) (bFromSweep :type Boolean) (SweepResult :type Hit%20Result%20Structure%20%28by%20ref%29))
  (if (Utilities|DoesObjectImplementInterface OtherActor "/Game/Blueprints/Weapons/I_HoldableCharacter.I_HoldableCharacter_C")
    (Utilities|Casting|CastToI_HoldableCharacter OtherActor)))

(event OnComponentEndOverlap(OperationRange)
  (params (OverlappedComponent :type Primitive%20Component%20Object%20Reference) (OtherActor :type Actor%20Object%20Reference) (OtherComp :type Primitive%20Component%20Object%20Reference) (OtherBodyIndex :type Integer))
  (if (Utilities|DoesObjectImplementInterface OtherActor "/Game/Blueprints/Weapons/I_HoldableCharacter.I_HoldableCharacter_C")
    (Utilities|Casting|CastToI_HoldableCharacter OtherActor)
    (Class|BlueprintImplementableInterface|OnPickup)))

(event Custom|Client%20Play%20sound
  (Audio|PlaySoundatLocation "/Game/ArtMaterials/MilitaryWeapSilver/Sound/Rifle/Cues/Rifle_Reload_Cue.Rifle_Reload_Cue" (Transformation|GetWorldLocation (Variables|Default|GetAssaultRifle_Pickup)) "0, 0, 0" 1.0 1.0 0.0 0 0 0))

(event Custom|Handle%20Pickup
  (params (Action%20Character :type Character%20Object%20Reference))
  (bind _astestive_character_bp (Utilities|Casting|CastToTestiveCharacter_BP Action%20Character))
  (Variables|/Game/Blueprints/Weapons/WeaponBase.WeaponBase_C|SetMag%20Remain (Variables|/Game/Blueprints/Characters/TestiveCharacter/TestiveCharacter_BP.TestiveCharacter_BP_C|GetWeapon _astestive_character_bp) (Variables|/Game/Blueprints/Weapons/WeaponBase.WeaponBase_C|GetMag%20Capacity (Variables|/Game/Blueprints/Characters/TestiveCharacter/TestiveCharacter_BP.TestiveCharacter_BP_C|GetWeapon _astestive_character_bp)))
  (CallFunction|ClientPlaySound))

(event EventBeginPlay)

(event Collision|EventActorBeginOverlap
  (params (OtherActor :type Actor%20Object%20Reference)))

(event EventTick
  (params (DeltaSeconds :type Float%20%28single-precision%29)))

(event EventOnPickup
  (params (ActionCharacter :type Character%20Object%20Reference)))

(fn ConstructionScript)

(fn GetPickableInfo
  (return ""))

(fn IsOpenforPickup
  (return false))