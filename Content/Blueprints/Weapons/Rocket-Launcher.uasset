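; Rocket launcher weapon Blueprint, a child of a parent weapon class, shown as an "RPG" pickup.
; The fire-effect event plays the launcher's fire animation on the weapon body when fired, otherwise a reload-detach sound at the fire arrow.
; The construction script runs the parent's, then fills the magazine to capacity.
; GetPickableInfo supplies the icon, title, Chinese description and quantity for pickup display.
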(event EventBeginPlay)

(event Collision|EventActorBeginOverlap
  (params (OtherActor :type Actor%20Object%20Reference)))

(event EventTick
  (params (DeltaSeconds :type Float%20%28single-precision%29)))

(event EventMakeFireEffectBP
  (params (Fired :type Boolean))
  (if Fired
    (Components|Animation|PlayAnimation (Variables|Default|GetWeaponBody) "/Game/ArtMaterials/MilitaryWeapSilver/Weapons/Animations/Fire_RocketLauncher_W.Fire_RocketLauncher_W" false)
    (else
      (Audio|PlaySoundatLocation "/Game/ArtMaterials/MilitaryWeapSilver/Sound/RocketLauncher/Cues/RocketLauncher_ReloadDetach_Cue.RocketLauncher_ReloadDetach_Cue" (Transformation|GetWorldLocation (Variables|Default|GetWeaponFireArrow)) "0, 0, 0" 1.0 1.0 0.0 0 0 0))))

(fn ConstructionScript
  (|CallParentFunction)
  (Variables|Default|SetMagRemain (Variables|Default|GetMagCapacity)))

(fn GetPickableInfo
  (return (Utilities|Struct|MakePickableItemDisplayData "/Game/Textures/Icons/controllerIconSprite_Sprite_3.controllerIconSprite_Sprite_3" "RPG" "火箭发射器" false 1)))