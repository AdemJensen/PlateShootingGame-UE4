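; Assault rifle weapon Blueprint, a 5.56mm hitscan pickup built on a parent weapon class.
; Each shot consumes one round and line-traces along the aim direction, or plays a sound and stops firing when empty.
; Hits trigger camera shake, weapon animation, physics impulse and damage, doubled for characters hit at neck_01 or its child bones.
; Impact sounds and particles are chosen by casting the physical material to surface classes.
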(event Custom|Server%20Handle%20Fire%20Actions
  (bind _weapondirection (Variables|Default|GetWeaponDirection))
  (bind _aiming_direction_vector (Variables|Default|GetAiming%20Direction%20Vector))
  (bind _returnvalue (Transformation|GetWorldLocation _weapondirection))
  (bind _returnvalue_2 (Math|Vector|Normalize _aiming_direction_vector))
  (bind (_outhit _returnvalue_3) (Collision|LineTraceByChannel (+ _returnvalue (* _returnvalue_2 6.0)) (+ _returnvalue (* _returnvalue_2 (Variables|Settings|GetShooting%20Range))) "TraceTypeQuery1" false 0 "None"))
  (if _returnvalue_3
    (CallFunction|ClientHitEffects (.PhysMat (Collision|BreakHitResult _outhit)) (.ImpactPoint (Collision|BreakHitResult _outhit)))
    (CallFunction|ClientApplyImpulse (.HitComponent (Collision|BreakHitResult _outhit)) (.Normal (Collision|BreakHitResult _outhit)) (.ImpactPoint (Collision|BreakHitResult _outhit)) (.HitBoneName (Collision|BreakHitResult _outhit)))
    (CallFunction|ServerApplyDamage (.HitActor (Collision|BreakHitResult _outhit)) (.HitBoneName (Collision|BreakHitResult _outhit)))))

(event Custom|Client%20Hit%20Effects
  (params (Physics%20Mat :type Physical%20Material%20Object%20Reference) (Location :type Vector))
  (bind _hit_sound (CallFunction|GetHitSound Physics%20Mat))
  (Audio|PlaySoundatLocation _hit_sound Location "0, 0, 0" 1.0 1.0 0.0 0 0 0)
  (bind _partical_sys (CallFunction|GetHitParticalSystem Physics%20Mat))
  (Effects|SpawnEmitteratLocation _partical_sys Location)
  (Components|Animation|PlayAnimation (Variables|Default|GetWeaponBody) "/Game/ArtMaterials/MilitaryWeapSilver/Weapons/Animations/Fire_Rifle_W.Fire_Rifle_W" false)
  (Camera|PlayWorldCameraShake "/Game/Blueprints/CamShake_01.CamShake_01_C" (Transformation|GetWorldLocation (Variables|Default|GetWeaponDirection)) 0.0 5e+02 3.0))

(event Custom|Client%20Apply%20Impulse
  (params (Impulse%20Target :type Primitive%20Component%20Object%20Reference) (Impulse :type Vector) (Impact%20Point :type Vector) (Bone%20Name :type Name))
  (if (and (Physics|IsSimulatingPhysics Impulse%20Target Bone%20Name) (Utilities|Enum|Equal(Enum) (Variables|/Script/Engine.SceneComponent|GetMobility Impulse%20Target) "Movable"))
    (Physics|AddImpulseatLocation Impulse%20Target (* Impulse (Variables|设置|GetShot%20Impulse)) Impact%20Point Bone%20Name)))

(event Custom|Server%20Apply%20damage
  (params (Damage%20target :type Actor%20Object%20Reference) (Hit%20Bone :type Name))
  (bind _damage_per_fire (Variables|Default|GetDamage%20Per%20Fire))
  (bind _ascharacter (Utilities|Casting|CastToCharacter Damage%20target)
    (:then
      ;[1 1 1] Apply damage ro character
      (Game|Damage|ApplyDamage Damage%20target (Math|Float|SelectFloat (* _damage_per_fire 2.0) _damage_per_fire (or (Utilities|Name|Equal(Name) Hit%20Bone "neck_01") (Class|SkinnedMeshComponent|BoneIsChildOf (Variables|/Script/Engine.Character|GetMesh _ascharacter) Hit%20Bone "neck_01"))) (Pawn|GetController (Variables|Default|GetWeaponOwner)) self))
    (:CastFailed
      ;[1 1 1] Apply damage to None character
      (Game|Damage|ApplyDamage Damage%20target (Variables|Default|GetDamage%20Per%20Fire) (Pawn|GetController (Variables|Default|GetWeaponOwner)) self))))

(event EventBeginPlay
  (|CallParentFunction) ; 此节点被禁用，将不会被调用。\n从引脚连出引线来编译功能。
)

(event Collision|EventActorBeginOverlap
  (params (OtherActor :type Actor%20Object%20Reference))
  (|CallParentFunction OtherActor) ; 此节点被禁用，将不会被调用。\n从引脚连出引线来编译功能。
)

(event EventTick
  (params (DeltaSeconds :type Float%20%28single-precision%29))
  (|CallParentFunction DeltaSeconds) ; 此节点被禁用，将不会被调用。\n从引脚连出引线来编译功能。
)

(event EventOnFire
  (bind _actual_use (CallFunction|UseAmmo 1 false))
  (if (> _actual_use 0)
    (CallFunction|ServerHandleFireActions)
    (else
      (Audio|PlaySoundatLocation "/Game/ArtMaterials/MilitaryWeapSilver/Sound/Rifle/Cues/Rifle_AmmoPickup_Cue.Rifle_AmmoPickup_Cue" (Transformation|GetWorldLocation (Variables|Default|GetWeaponBody)) "0, 0, 0" 1.0 1.0 0.0 0 0 0)
      (CallFunction|ActionStopFire))))

(event EventOnDrop
  (|CallParentFunction))

(event EventOnPickup
  (params (Action%20Character :type Character%20Object%20Reference))
  (|CallParentFunction Action%20Character))

(fn ConstructionScript
  (|CallParentFunction))

(fn GetPickableInfo
  (return (Utilities|Struct|MakePickableItemDisplayData "/Game/Textures/Icons/controllerIconSprite_Sprite_3.controllerIconSprite_Sprite_3" "突击步枪" "使用5.56mm子弹" false 1)))

(fn GetHitSound
  (params (Phy%20Mat%20inst :type Physical%20Material%20Object%20Reference))
  (Utilities|FlowControl|Sequence
    (:then_0
      (Utilities|Casting|CastToMetal Phy%20Mat%20inst)
      (return "/Game/Audio/Bullet_Impact/BI_Metal_Heavy.BI_Metal_Heavy"))
    (:then_1
      (Utilities|Casting|CastToBrick Phy%20Mat%20inst)
      (return "/Game/Audio/Bullet_Impact/BI_Brick_Heavy.BI_Brick_Heavy"))
    (:then_2
      (Utilities|Casting|CastToDirt Phy%20Mat%20inst)
      (return "/Game/Audio/Bullet_Impact/BI_Dirt_Heavy.BI_Dirt_Heavy"))
    (:then_3
      (Utilities|Casting|CastToGlass Phy%20Mat%20inst)
      (return "/Game/Audio/Bullet_Impact/BI_Glass_Heavy.BI_Glass_Heavy"))
    (:then_4
      (Utilities|Casting|CastToWood Phy%20Mat%20inst)
      (return "/Game/Audio/Bullet_Impact/BI_Wood_Heavy.BI_Wood_Heavy"))
    (:then_5
      (Utilities|Casting|CastToFlesh Phy%20Mat%20inst)
      (return "/Game/ArtMaterials/Bullet_Impact_Sounds/Cues/bullet_impact_body_flesh_01_Cue.bullet_impact_body_flesh_01_Cue"))
    (:then_6
      (return 0))))

(fn GetHitParticalSystem
  (params (Phy%20mat :type Physical%20Material%20Object%20Reference))
  (Utilities|FlowControl|Sequence
    (:then_0
      (Utilities|Casting|CastToMetal Phy%20mat)
      (return "/Game/ArtMaterials/MilitaryWeapSilver/FX/P_Impact_Metal_Medium_01.P_Impact_Metal_Medium_01"))
    (:then_1
      (Utilities|Casting|CastToBrick Phy%20mat)
      (return "/Game/ArtMaterials/MilitaryWeapSilver/FX/P_Impact_Stone_Medium_01.P_Impact_Stone_Medium_01"))
    (:then_2
      (Utilities|Casting|CastToDirt Phy%20mat)
      (return "/Game/ArtMaterials/MilitaryWeapSilver/FX/P_Impact_Stone_Large_01.P_Impact_Stone_Large_01"))
    (:then_3
      (Utilities|Casting|CastToGlass Phy%20mat)
      (return "/Game/Effects/P_Hit.P_Hit"))
    (:then_4
      (Utilities|Casting|CastToWood Phy%20mat)
      (return "/Game/ArtMaterials/MilitaryWeapSilver/FX/P_Impact_Wood_Medium_01.P_Impact_Wood_Medium_01"))
    (:then_5
      (Utilities|Casting|CastToFlesh Phy%20mat)
      (return "/Game/Effects/P_Hit_Blood.P_Hit_Blood"))
    (:then_6
      (return "/Game/Effects/P_Hit.P_Hit"))))