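; Grenade launcher weapon that can be picked up and fires physics-driven explosive projectiles using its own grenade ammo.
; On fire it consumes one round, plays the weapon animation, spawns a projectile configured with damage and radius, then launches it by impulse along the aim direction.
; Without ammo it plays a sound and stops firing.
; It also supplies pickup display info and heavy impact sounds chosen by physical material.
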(event EventBeginPlay
  (|CallParentFunction) ; 此节点被禁用，将不会被调用。\n从引脚连出引线来编译功能。
)

(event Collision|EventActorBeginOverlap
  (params (OtherActor :type Actor%20Object%20Reference))
  (|CallParentFunction OtherActor) ; 此节点被禁用，将不会被调用。\n从引脚连出引线来编译功能。
)

(event EventTick
  (params (DeltaSeconds :type Float%20%28single-precision%29))
  (|CallParentFunction DeltaSeconds) ; 此节点被禁用，将不会被调用。\n从引脚连出引线来编译功能。
)

(event EventOnFire
  (bind _actual_use (CallFunction|UseAmmo 1 false))
  (if (> _actual_use 0)
    (Components|Animation|PlayAnimation (Variables|Default|GetWeaponBody) "/Game/ArtMaterials/MilitaryWeapSilver/Weapons/Animations/Fire_GrenadeLauncher_W.Fire_GrenadeLauncher_W" false)
    (bind _returnvalue (Game|SpawnActorfromClass "/Game/Blueprints/Weapons/GrenadeLauncherProjectile.GrenadeLauncherProjectile_C" (Math|Transform|MakeTransform (Transformation|GetWorldLocation (Variables|Default|GetWeaponDirection)) (CallFunction|GetWeaponTowardsRotation) (Transformation|GetWorldScale (Variables|Default|GetWeaponBody))) "Undefined" self (Variables|Default|GetWeaponOwner)))
    (Default|Configure _returnvalue (Variables|Default|GetBase%20Damage) (Variables|Default|GetDamage%20Radius) self)
    (Physics|AddImpulse (Variables|/Game/Blueprints/Weapons/GrenadeLauncherProjectile.GrenadeLauncherProjectile_C|GetProjectile _returnvalue) (* (Math|Rotator|GetRotationXVector (CallFunction|GetWeaponTowardsRotation)) (Variables|Default|GetInitial%20Impulse%20Rate)) "None" false)
    (else
      (Audio|PlaySoundatLocation "/Game/ArtMaterials/MilitaryWeapSilver/Sound/Rifle/Cues/Rifle_AmmoPickup_Cue.Rifle_AmmoPickup_Cue" (Transformation|GetWorldLocation (Variables|Default|GetWeaponBody)) "0, 0, 0" 1.0 1.0 0.0 0 0 0)
      (CallFunction|StopFire))))

(event EventOnDrop
  (|CallParentFunction))

(event EventOnPickup
  (params (Action%20Character :type Character%20Object%20Reference))
  (|CallParentFunction Action%20Character))

(fn ConstructionScript
  (|CallParentFunction))

(fn GetPickableInfo
  (return (Utilities|Struct|MakePickableItemDisplayData "/Game/Textures/Icons/dice.dice" "榴弹发射器" "使用特殊弹药（榴弹）" false 1)))

(fn GetHitSound
  (params (Phy%20Mat%20inst :type Physical%20Material%20Object%20Reference))
  (Utilities|FlowControl|Sequence
    (:then_0
      (Utilities|Casting|CastToMetal Phy%20Mat%20inst)
      (return "/Game/Audio/Bullet_Impact/BI_Metal_Heavy.BI_Metal_Heavy"))
    (:then_1
      (Utilities|Casting|CastToBrick Phy%20Mat%20inst)
      (return "/Game/Audio/Bullet_Impact/BI_Brick_Heavy.BI_Brick_Heavy"))
    (:then_2
      (Utilities|Casting|CastToDirt Phy%20Mat%20inst)
      (return "/Game/Audio/Bullet_Impact/BI_Dirt_Heavy.BI_Dirt_Heavy"))
    (:then_3
      (Utilities|Casting|CastToGlass Phy%20Mat%20inst)
      (return "/Game/Audio/Bullet_Impact/BI_Glass_Heavy.BI_Glass_Heavy"))
    (:then_4
      (Utilities|Casting|CastToWood Phy%20Mat%20inst)
      (return "/Game/Audio/Bullet_Impact/BI_Wood_Heavy.BI_Wood_Heavy"))
    (:then_5
      (Utilities|Casting|CastToFlesh Phy%20Mat%20inst)
      (return "/Game/ArtMaterials/Bullet_Impact_Sounds/Cues/bullet_impact_body_flesh_01_Cue.bullet_impact_body_flesh_01_Cue"))
    (:then_6
      (return 0))))