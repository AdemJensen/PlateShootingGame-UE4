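; Ammo pickup actor (legacy "Old_" asset) that refills the magazine of the picking character's weapon.
; OperationRange overlaps tell Old_HoldableCharacter actors when the item becomes available or is lost.
; OnPickup routes through HandlePickup, which casts to TestiveCharacter_BP, sets MagRemain to MagCapacity and plays a reload sound, without destroying the pickup.
; It supplies display info for pickup UI, while IsOpenForPickup always returns false.
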(event OnComponentBeginOverlap(OperationRange)
  (params (OverlappedComponent :type Primitive%20Component%20Object%20Reference) (OtherActor :type Actor%20Object%20Reference) (OtherComp :type Primitive%20Component%20Object%20Reference) (OtherBodyIndex :type Integer) (bFromSweep :type Boolean) (SweepResult :type Hit%20Result%20Structure%20%28by%20ref%29))
  (if (Utilities|DoesObjectImplementInterface OtherActor "/Game/Blueprints/Weapons/Old_HoldableCharacter.Old_HoldableCharacter_C")
    (bind _asold_holdable_character (Utilities|Casting|CastToOld_HoldableCharacter OtherActor))
    (Default|OnAbletoPickItem _asold_holdable_character self)))

(event OnComponentEndOverlap(OperationRange)
  (params (OverlappedComponent :type Primitive%20Component%20Object%20Reference) (OtherActor :type Actor%20Object%20Reference) (OtherComp :type Primitive%20Component%20Object%20Reference) (OtherBodyIndex :type Integer))
  (if (Utilities|DoesObjectImplementInterface OtherActor "/Game/Blueprints/Weapons/Old_HoldableCharacter.Old_HoldableCharacter_C")
    (bind _asold_holdable_character (Utilities|Casting|CastToOld_HoldableCharacter OtherActor))
    (Default|OnLostTrackonItem _asold_holdable_character self)))

(event Custom|Client%20Play%20sound
  (Audio|PlaySoundatLocation "/Game/ArtMaterials/MilitaryWeapSilver/Sound/Rifle/Cues/Rifle_Reload_Cue.Rifle_Reload_Cue" (Transformation|GetWorldLocation (Variables|Default|GetAssaultRifle_Pickup)) "0, 0, 0" 1.0 1.0 0.0 0 0 0))

(event Custom|Handle%20Pickup
  (params (Action%20Character :type Character%20Object%20Reference))
  (bind _astestive_character_bp (Utilities|Casting|CastToTestiveCharacter_BP Action%20Character))
  (Variables|/Game/Blueprints/Weapons/Old_WeaponBase.Old_WeaponBase_C|SetMag%20Remain (Variables|/Game/Blueprints/Characters/TestiveCharacter/TestiveCharacter_BP.TestiveCharacter_BP_C|GetWeapon _astestive_character_bp) (Variables|/Game/Blueprints/Weapons/Old_WeaponBase.Old_WeaponBase_C|GetMag%20Capacity (Variables|/Game/Blueprints/Characters/TestiveCharacter/TestiveCharacter_BP.TestiveCharacter_BP_C|GetWeapon _astestive_character_bp)))
  (CallFunction|ClientPlaySound))

(event EventBeginPlay)

(event Collision|EventActorBeginOverlap
  (params (OtherActor :type Actor%20Object%20Reference)))

(event EventTick
  (params (DeltaSeconds :type Float%20%28single-precision%29)))

(event EventOnPickup
  (params (Action%20Character :type Character%20Object%20Reference))
  (CallFunction|HandlePickup Action%20Character))

(fn ConstructionScript)

(fn GetPickableInfo
  (return (Utilities|Struct|MakePickableItemDisplayData "/Game/Textures/Icons/controllerIconSprite_Sprite_5.controllerIconSprite_Sprite_5" "弹药" "各种弹药" false 1)))

(fn IsOpenforPickup
  (return false))