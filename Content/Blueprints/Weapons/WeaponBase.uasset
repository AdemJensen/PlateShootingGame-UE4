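; Base weapon actor that characters can pick up, drop, fire and reload, with action events meant for child implementation.
; A Tick timer paces OnFire by FireRate for single or continuous fire, while UseAmmo handles magazine consumption.
; PickupRange tracks overlapping HoldableCharacters and notifies them as availability changes; pickup and drop toggle body physics.
; OnFire only prints placeholder text, and nothing here refills the magazine.
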(event OnComponentBeginOverlap(PickupRange)
  (params (OverlappedComponent :type Primitive%20Component%20Object%20Reference) (OtherActor :type Actor%20Object%20Reference) (OtherComp :type Primitive%20Component%20Object%20Reference) (OtherBodyIndex :type Integer) (bFromSweep :type Boolean) (SweepResult :type Hit%20Result%20Structure%20%28by%20ref%29))
  (if (Utilities|DoesObjectImplementInterface OtherActor "/Game/Blueprints/Weapons/HoldableCharacter.HoldableCharacter_C")
    (bind _asholdable_character (Utilities|Casting|CastToHoldableCharacter OtherActor))
    (Utilities|Array|Add (Variables|Status|GetCharacters%20Waiting%20to%20me%20pickup) _asholdable_character)
    (if (not (Utilities|IsValid (Variables|设置|GetWeaponOwner)))
      (Default|OnAbletoPickItem _asholdable_character self))))

(event OnComponentEndOverlap(PickupRange)
  (params (OverlappedComponent :type Primitive%20Component%20Object%20Reference) (OtherActor :type Actor%20Object%20Reference) (OtherComp :type Primitive%20Component%20Object%20Reference) (OtherBodyIndex :type Integer))
  (if (Utilities|DoesObjectImplementInterface OtherActor "/Game/Blueprints/Weapons/HoldableCharacter.HoldableCharacter_C")
    (bind _asholdable_character (Utilities|Casting|CastToHoldableCharacter OtherActor))
    (bind _returnvalue (Utilities|Array|RemoveItem (Variables|Status|GetCharacters%20Waiting%20to%20me%20pickup) _asholdable_character))
    (if _returnvalue
      (Default|OnLostTrackonItem _asholdable_character self))))

(event EventBeginPlay)

(event Collision|EventActorBeginOverlap
  (params (OtherActor :type Actor%20Object%20Reference)))

(event EventTick
  (params (DeltaSeconds :type Float%20%28single-precision%29))
  ;[1 1 1] Fire
  (if (< (Variables|Status|GetTime%20Since%20Last%20Fire) (* 2 (Variables|Settings|GetFire%20Rate)))
    (Variables|Status|SetTime%20Since%20Last%20Fire (+ DeltaSeconds (Variables|Status|GetTime%20Since%20Last%20Fire))))
  (if (Variables|Status|GetIs%20Firing)
    (if (> (Variables|Status|GetTime%20Since%20Last%20Fire) (Variables|Settings|GetFire%20Rate))
      (Variables|Status|SetTime%20Since%20Last%20Fire (Math|Float|%(Float) (Variables|Status|GetTime%20Since%20Last%20Fire) (Variables|Settings|GetFire%20Rate)))
      (CallFunction|OnFire)
      (if (not (Variables|设置|GetFire%20Continuously))
        (CallFunction|StopFire)))))

(event EventOnPickup
  (params (Action%20Character :type Character%20Object%20Reference))
  (bind _weaponbody (Variables|Default|GetWeaponBody))
  (Variables|设置|SetWeaponOwner Action%20Character)
  (Physics|SetSimulatePhysics _weaponbody false)
  (Physics|SetEnableGravity _weaponbody false)
  (for _array_element (Variables|Status|GetCharacters%20Waiting%20to%20me%20pickup)
    (Default|OnLostTrackonItem _array_element self)))

(event EventOnDrop
  (bind _weaponbody (Variables|Default|GetWeaponBody))
  (Variables|设置|SetWeaponOwner 0)
  (Physics|SetSimulatePhysics _weaponbody true)
  (Physics|SetEnableGravity _weaponbody true)
  (for _array_element (Variables|Status|GetCharacters%20Waiting%20to%20me%20pickup)
    (Default|OnAbletoPickItem _array_element self)))

(event Custom|On%20Fire
  (Development|PrintText "Hello"))

(event Custom|On%20Reload%20Interrupt)

(event Custom|On%20Reload%20Start)

(event Custom|On%20Reload%20Complete)

(fn ConstructionScript
  (Variables|Status|SetTime%20Since%20Last%20Fire (Variables|Settings|GetFire%20Rate)))

(fn Fire
  (if (not (Variables|Status|GetIs%20Firing))
    (if (Variables|Status|GetIs%20Reloading)
      (if (<= (Variables|Status|GetMag%20Remain) 0)
        (return false)
        (else
          (CallFunction|StopReload true))))
    (Variables|Status|SetIs%20Firing true)
    (return true)))

(fn StopFire
  (Variables|Status|SetIs%20Firing false))

(fn Reload
  (if (or (Variables|Status|GetIs%20Reloading) (not (Variables|设置|GetNeeds%20Reload)))
    (return false)
    (elif (>= (Variables|Status|GetMag%20Remain) (Variables|设置|GetMag%20Capacity))
      (return false)
      (else
        (Variables|Status|SetIs%20Reloading true)
        (Variables|Status|SetIs%20Firing false)
        (CallFunction|OnReloadStart)
        (return true)))))

(fn StopReload
  (params (Generate%20Interruption :type Boolean))
  (if (Variables|Status|GetIs%20Reloading)
    (Variables|Status|SetIs%20Reloading false)
    (CallFunction|OnReloadInterrupt)
    (if Generate%20Interruption
      (Default|CallOnReloadInterrupted))))

(fn GetWeaponFireLocation
  (return (Transformation|GetWorldLocation (Variables|Default|GetWeaponDirection))))

(fn GetWeaponTowardsRotation
  (return (Transformation|GetWorldRotation (Variables|Default|GetWeaponDirection))))

(fn SetFireRotation
  (params (Aiming%20Rotation :type Rotator))
  (Variables|设置|SetAiming%20Direction%20Vector (Math|Rotator|GetRotationXVector Aiming%20Rotation)))

(fn UseAmmo
  (params (Expected%20Ammo :type Integer) (Can%20use%20parcial :type Boolean))
  (if (Variables|设置|GetNeeds%20Reload)
    (if Can%20use%20parcial
      (if (>= (Variables|Status|GetMag%20Remain) Expected%20Ammo)
        _
        (else
          (LocalVariables|SetMag%20Use (Variables|Status|GetMag%20Remain))
          (Variables|Status|SetMag%20Remain 0)
          (return (LocalVariables|GetMag%20Use))))
      (elif (>= (Variables|Status|GetMag%20Remain) Expected%20Ammo)
        _
        (else
          (return 0))))
    (Variables|Status|SetMag%20Remain (- (Variables|Status|GetMag%20Remain) Expected%20Ammo))
    (return Expected%20Ammo)
    (else
      (return Expected%20Ammo))))

(fn GetPickableInfo
  (return ""))

(fn IsOpenforPickup
  (return (Utilities|IsValid (Variables|设置|GetWeaponOwner))))