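; AW-50 sniper rifle weapon Blueprint, supplying effects, scope behavior and pickup display info on top of its parent class.
; Its camera copies the owner's camera rotation every tick and sets fire direction.
; Firing animates the body and draws a Niagara beam to a line-trace endpoint; hits choose sound and particles by physical material and shake the camera.
; Scope events toggle the HUD overlay, while a timeline smoothly steps through zoom FOVs.
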(event EventBeginPlay
  (|CallParentFunction))

(event Collision|EventActorBeginOverlap
  (params (OtherActor :type Actor%20Object%20Reference))
  (|CallParentFunction OtherActor))

(event EventTick
  (params (DeltaSeconds :type Float%20%28single-precision%29))
  (bind _weaponowner (Variables|Default|GetWeaponOwner))
  (|CallParentFunction DeltaSeconds)
  ;[1 1 1] Sync gun camera rotation.
  (Utilities|IsValid _weaponowner
    (:Is%20Valid
      (bind _asshooter_game_character_base (Utilities|Casting|CastToShooterGameCharacterBase _weaponowner))
      (Transformation|SetWorldRotation (Variables|Default|GetCamera) (Transformation|GetWorldRotation (Variables|/Script/PlateShootingGame.ShooterGameCharacterBase|GetCamera _asshooter_game_character_base)) false true))))

(event EventMakeFireEffectBP
  (params (Fired :type Boolean))
  (bind _weaponfirearrow (Variables|Default|GetWeaponFireArrow))
  (bind _weaponfirearrow_2 (Variables|Default|GetWeaponFireArrow))
  (bind _firedirection (Variables|Default|GetFireDirection))
  (bind _shootingrange (Variables|Default|GetShootingRange))
  (bind _returnvalue (Transformation|GetWorldLocation _weaponfirearrow))
  (bind _returnvalue_2 (Transformation|GetWorldLocation _weaponfirearrow_2))
  (bind _returnvalue_3 (* _firedirection _shootingrange))
  (bind _returnvalue_4 (+ _returnvalue _returnvalue_3))
  (if Fired
    (Components|Animation|PlayAnimation (Variables|Default|GetWeaponBody) "/Game/ArtMaterials/MilitaryWeapSilver/Weapons/Animations/Fire_SniperRifle_W.Fire_SniperRifle_W" false)
    (bind _returnvalue_5 (Niagara|SpawnSystematLocation "/Game/Effects/NG_BulletLine.NG_BulletLine" _returnvalue_2))
    (bind (_outhit _returnvalue_6) (Collision|LineTraceByChannel _returnvalue_2 _returnvalue_4 "TraceTypeQuery1" true 0 "None" true "(R=1.000000,G=0.000000,B=0.000000,A=1.000000)" "(R=0.000000,G=1.000000,B=0.000000,A=1.000000)" 2.0))
    (Effects|Components|ParticleSystem|SetVectorParameter _returnvalue_5 "Beam End" (Math|Vector|SelectVector (.Location (Collision|BreakHitResult _outhit)) _returnvalue_4 _returnvalue_6))
    (Effects|Components|ParticleSystem|SetFloatParameter _returnvalue_5 "Beam Width" 4.0)
    (Effects|Components|ParticleSystem|SetFloatParameter _returnvalue_5 "Lifetime" 1.0)
    (else
      (Audio|PlaySoundatLocation "/Game/ArtMaterials/MilitaryWeapSilver/Sound/SniperRifle/Cues/SniperRifle_AmmoPickup_Cue.SniperRifle_AmmoPickup_Cue" (Transformation|GetWorldLocation (Variables|Default|GetWeaponBody)) "0, 0, 0" 1.0 1.0 0.0 0 0 0))))

(event EventMakeHitEffectBP
  (params (HitPhysicalMaterial :type Physical%20Material%20Object%20Reference) (HitLocation :type Vector :default "0, 0, 0") (HitActor :type Actor%20Object%20Reference) (HitComponent :type Primitive%20Component%20Object%20Reference) (HitBoneName :type Name :default "None"))
  (bind (_partical_sys _sound_cue) (CallFunction|GetHitEffects HitPhysicalMaterial))
  (Audio|PlaySoundatLocation _sound_cue HitLocation "0, 0, 0" 1.0 1.0 0.0 0 0 0)
  (Effects|SpawnEmitteratLocation _partical_sys HitLocation)
  (Camera|PlayWorldCameraShake "/Game/Blueprints/CamShake_01.CamShake_01_C" (Transformation|GetWorldLocation (Variables|Default|GetWeaponFireArrow)) 0.0 5e+02 3.0))

(event EventOnEnterScopeBP
  (params (Character :type Shooter%20Game%20Character%20Base%20Object%20Reference) (Weapon :type Weapon%20Object%20Reference))
  (Audio|PlaySound2D "/Game/ArtMaterials/MilitaryWeapSilver/Sound/SniperRifle/Cues/SniperRifle_ZoomIn_Cue.SniperRifle_ZoomIn_Cue" 1.0 1.0 0.0 0 0)
  (bind _foundwidgets (Widget|GetAllWidgetsOfClass "/Game/Blueprints/Widgets/MyHUD.MyHUD_C" true))
  (Default|ToggleSinperScope (Utilities|Array|Get(acopy) _foundwidgets) true))

(event EventOnExitScopeBP
  (params (Character :type Shooter%20Game%20Character%20Base%20Object%20Reference) (Weapon :type Weapon%20Object%20Reference))
  (Audio|PlaySound2D "/Game/ArtMaterials/MilitaryWeapSilver/Sound/SniperRifle/Cues/SniperRifle_ZoomOut_Cue.SniperRifle_ZoomOut_Cue" 1.0 1.0 0.0 0 0)
  (bind _foundwidgets (Widget|GetAllWidgetsOfClass "/Game/Blueprints/Widgets/MyHUD.MyHUD_C" true))
  (Default|ToggleSinperScope (Utilities|Array|Get(acopy) _foundwidgets) false))

(event EventSetFireDirectionbyAimParameters
  (params (Character :type Shooter%20Game%20Character%20Base%20Object%20Reference) (Weapon :type Weapon%20Object%20Reference))
  (bind _camera (Variables|Default|GetCamera))
  (Class|Weapon|SetFireDirectionbyCameraParameters (Transformation|GetWorldLocation _camera) (Transformation|GetWorldRotation _camera)))

(event EventOnAdjustScope
  (params (Character :type Shooter%20Game%20Character%20Base%20Object%20Reference) (Weapon :type Weapon%20Object%20Reference))
  (bind _currentscopefov (Variables|Default|GetCurrentScopeFOV))
  (bind _scopefov (Variables|Default|GetScopeFOV))
  (Math|Integer|IncrementInt (Variables|Default|GetCurrentScopeFOV)
    (:%20%20
      (Audio|PlaySound2D "/Game/ArtMaterials/MilitaryWeapSilver/Sound/SniperRifle/Cues/SniperRifle_ZoomIn_Cue.SniperRifle_ZoomIn_Cue" 1.0 1.0 0.0 0 0)
      (bind _fov_percentage (Timeline|Adjust%20FOV PlayFromStart)
        (:Update
          (Camera|SetFieldOfView (Variables|Default|GetCamera) (Math|Float|Lerp (Utilities|Array|Get(acopy) _scopefov (- _currentscopefov 1)) (Utilities|Array|Get(acopy) _scopefov _currentscopefov) _fov_percentage)))))))

(fn ConstructionScript
  (|CallParentFunction)
  (Variables|Default|SetMagRemain (Variables|Default|GetMagCapacity)))

(fn GetPickableInfo
  (return (Utilities|Struct|MakePickableItemDisplayData "/Game/Textures/Icons/controllerIconSprite_Sprite_3.controllerIconSprite_Sprite_3" "AW-50 Precosion Rifle" "英国产AW-50高精度狙击步枪" false 1)))

(fn GetHitEffects
  (params (Phys%20Mat :type Object%20Object%20Reference))
  (Utilities|FlowControl|Sequence
    (:then_0
      (Utilities|Casting|CastToMetal Phys%20Mat)
      (return "/Game/ArtMaterials/MilitaryWeapSilver/FX/P_Impact_Metal_Medium_01.P_Impact_Metal_Medium_01" "/Game/Audio/Bullet_Impact/BI_Metal_Heavy.BI_Metal_Heavy"))
    (:then_1
      (Utilities|Casting|CastToBrick Phys%20Mat)
      (return "/Game/ArtMaterials/MilitaryWeapSilver/FX/P_Impact_Stone_Medium_01.P_Impact_Stone_Medium_01" "/Game/Audio/Bullet_Impact/BI_Brick_Heavy.BI_Brick_Heavy"))
    (:then_2
      (Utilities|Casting|CastToDirt Phys%20Mat)
      (return "/Game/ArtMaterials/MilitaryWeapSilver/FX/P_Impact_Stone_Large_01.P_Impact_Stone_Large_01" "/Game/Audio/Bullet_Impact/BI_Dirt_Heavy.BI_Dirt_Heavy"))
    (:then_3
      (Utilities|Casting|CastToGlass Phys%20Mat)
      (return "/Game/Effects/P_Hit.P_Hit" "/Game/Audio/Bullet_Impact/BI_Glass_Heavy.BI_Glass_Heavy"))
    (:then_4
      (Utilities|Casting|CastToWood Phys%20Mat)
      (return "/Game/ArtMaterials/MilitaryWeapSilver/FX/P_Impact_Wood_Medium_01.P_Impact_Wood_Medium_01" "/Game/Audio/Bullet_Impact/BI_Wood_Heavy.BI_Wood_Heavy"))
    (:then_5
      (Utilities|Casting|CastToFlesh Phys%20Mat)
      (return "/Game/Effects/P_Hit_Blood.P_Hit_Blood" "/Game/ArtMaterials/Bullet_Impact_Sounds/Cues/bullet_impact_body_flesh_01_Cue.bullet_impact_body_flesh_01_Cue"))
    (:then_6
      (return "/Game/Effects/P_Hit.P_Hit" 0))))