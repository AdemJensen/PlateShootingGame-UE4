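; Grenade launcher projectile that bounces off surfaces and explodes for radial damage, configured with damage, radius and owning weapon.
; The server detonates it on hitting a Character or Target_BP, or when it slows after a one-second arming delay; any damage also detonates it.
; Other hits play throttled, surface-based bounce sounds from the weapon.
; Explosion spawns effects, then sphere-traces to push ragdolls, live characters and objects before destroying itself.
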(event OnComponentHit(Projectile)
  (params (HitComponent :type Primitive%20Component%20Object%20Reference) (OtherActor :type Actor%20Object%20Reference) (OtherComp :type Primitive%20Component%20Object%20Reference) (NormalImpulse :type Vector :default "0, 0, 0") (Hit :type Hit%20Result%20Structure%20%28by%20ref%29))
  (bind (_bblockinghit _binitialoverlap _time _distance _location _impactpoint _normal _impactnormal _physmat) (Collision|BreakHitResult Hit))
  (bind _weapon (Variables|设置|GetWeapon))
  (if (Networking|IsServer)
    (Utilities|Casting|CastToCharacter OtherActor
      (:then
        (CallFunction|Explode :!label _label))
      (:CastFailed
        (Utilities|Casting|CastToTarget_BP OtherActor
          (:then
            (goto _label))
          (:CastFailed
            (Utilities|IsValid _weapon
              (:Is%20Valid
                (if (Variables|Status|GetMake%20Hit%20Sound)
                  (bind _hit_sound (Default|GetHitSound _weapon _physmat))
                  (CallFunction|ClientMakeBounceSound _hit_sound _impactpoint)
                  (Variables|Status|SetMake%20Hit%20Sound false)
                  (Utilities|FlowControl|Delay 0.2)
                  (Variables|Status|SetMake%20Hit%20Sound true))))))))))

(event Custom|Explode
  (bind _self self)
  (if (not (Variables|Status|GetExploding)) ; Prevent infinite loops
    (Variables|Status|SetExploding true)
    (CallFunction|ProjectileExplodeEffects)
    (Game|Damage|ApplyRadialDamage (Variables|Settings|GetBase%20Damage) (Transformation|GetWorldLocation (Variables|Default|GetProjectile)) (Variables|Settings|GetDamage%20Radius) 0 0 _self (Game|GetInstigatorController _self) false "ECC_Visibility")
    (CallFunction|ClientMakeImpulse)))

(event Custom|On%20Activation
  (Variables|Status|SetActivated true))

(event Custom|Projectile%20Explode%20Effects
  (bind _projectile (Variables|Default|GetProjectile))
  (bind _projectile_2 (Variables|Default|GetProjectile))
  (bind _returnvalue (Transformation|GetWorldTransform _projectile_2))
  (bind _returnvalue_2 (Transformation|GetWorldTransform _projectile))
  (bind (_location _rotation _scale) (Math|Transform|BreakTransform _returnvalue))
  (bind (_location_2 _rotation_2) (Math|Transform|BreakTransform _returnvalue_2))
  (Effects|SpawnEmitteratLocation "/Game/ArtMaterials/MilitaryWeapSilver/FX/P_Grenade_Explosion_01.P_Grenade_Explosion_01" _location _rotation _scale)
  (Audio|PlaySoundatLocation "/Game/ArtMaterials/MilitaryWeapSilver/Sound/GrenadeLauncher/Cues/GrenadeLauncher_Explosion_Cue.GrenadeLauncher_Explosion_Cue" _location_2 _rotation_2 1.0 1.0 0.0 0 0 0))

(event Custom|Client%20Make%20Impulse
  (bind _projectile (Variables|Default|GetProjectile))
  (bind _returnvalue (Transformation|GetWorldLocation _projectile))
  (bind _outhits (Collision|MultiSphereTraceByChannel _returnvalue _returnvalue (Variables|设置|GetExplosion%20Blast%20Radius) "TraceTypeQuery2" false 0 "None"))
  (for _array_element _outhits
    (bind _as角色 (Utilities|Casting|CastToCharacter (.HitActor (Collision|BreakHitResult _array_element)))
      (:then
        (if (Physics|IsSimulatingPhysics (Variables|/Script/Engine.Character|GetMesh _as角色) "None")
          ;[1 1 1] Impact on dead character
          (Physics|AddRadialImpulse (Variables|/Script/Engine.Character|GetMesh _as角色) (Transformation|GetWorldLocation (Variables|Default|GetProjectile)) (Variables|Settings|GetDamage%20Radius) (Variables|设置|GetExplosion%20Blast%20Strength) "RIF_Constant" false)
          (else
            ;[1 1 1] Impact on live Character
            (Physics|AddImpulse (Variables|/Script/Engine.Character|GetCharacterMovement _as角色) (Utilities|CalcExplosionImpulseforCharacter (Transformation|GetWorldLocation (Variables|/Script/Engine.Character|GetCapsuleComponent _as角色)) (Transformation|GetWorldLocation (Variables|Default|GetProjectile))) false))))
      (:CastFailed
        ;[1 1 1] Impact On Moveable Objects
        (Physics|AddRadialImpulse (.HitComponent (Collision|BreakHitResult _array_element)) (Transformation|GetWorldLocation (Variables|Default|GetProjectile)) (Variables|Settings|GetDamage%20Radius) (Variables|设置|GetExplosion%20Blast%20Strength) "RIF_Constant" false))))
  (Actor|DestroyActor))

(event Custom|Client%20Make%20Bounce%20Sound
  (params (Sound :type Sound%20Base%20Object%20Reference) (Location :type Vector))
  (Audio|PlaySoundatLocation Sound Location "0, 0, 0" 1.0 1.0 0.0 0 0 0))

(event EventBeginPlay
  (Utilities|Time|SetTimerbyEvent (delegate Custom|On%20Activation) 1.0))

(event Collision|EventActorBeginOverlap
  (params (OtherActor :type Actor%20Object%20Reference)))

(event EventTick
  (params (DeltaSeconds :type Float%20%28single-precision%29))
  (if (Networking|IsServer)
    (if (and (< (Math|Vector|VectorLength (Transformation|GetVelocity)) 5e+01) (Variables|Status|GetActivated))
      (CallFunction|Explode))))

(event Game|Damage|EventAnyDamage
  (params (Damage :type Float%20%28single-precision%29) (DamageType :type Damage%20Type%20Object%20Reference) (InstigatedBy :type Controller%20Object%20Reference) (DamageCauser :type Actor%20Object%20Reference))
  (CallFunction|Explode))

(fn ConstructionScript)

(fn Configure
  (params (Base%20Damage :type Float%20%28single-precision%29) (Damage%20Radius :type Float%20%28single-precision%29) (Weapon :type Old%20Weapon%20Base%20Object%20Reference))
  (Variables|Settings|SetBase%20Damage Base%20Damage)
  (Variables|Settings|SetDamage%20Radius Damage%20Radius)
  (Variables|设置|SetWeapon Weapon))