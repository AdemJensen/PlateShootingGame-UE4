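; Assault rifle weapon Blueprint that fires hitscan shots and can be picked up and dropped, deferring both to its parent.
; Each shot uses one round, plays the fire animation and a camera shake, then line-traces along the aim direction.
; Hits play a body sound for Characters or a surface sound otherwise, spawn an impact effect and apply damage.
; Without ammo it plays a sound and stops firing; it also supplies its pickup display info.
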(event EventBeginPlay
  (|CallParentFunction) ; 此节点被禁用，将不会被调用。\n从引脚连出引线来编译功能。
)

(event Collision|EventActorBeginOverlap
  (params (OtherActor :type Actor%20Object%20Reference))
  (|CallParentFunction OtherActor) ; 此节点被禁用，将不会被调用。\n从引脚连出引线来编译功能。
)

(event EventTick
  (params (DeltaSeconds :type Float%20%28single-precision%29))
  (|CallParentFunction DeltaSeconds) ; 此节点被禁用，将不会被调用。\n从引脚连出引线来编译功能。
)

(event EventOnFire
  (bind _weapondirection (Variables|Default|GetWeaponDirection))
  (bind _aiming_direction_vector (Variables|Default|GetAiming%20Direction%20Vector))
  (bind _returnvalue (Transformation|GetWorldLocation _weapondirection))
  (bind _returnvalue_2 (Math|Vector|Normalize _aiming_direction_vector))
  (bind _actual_use (CallFunction|UseAmmo 1 false))
  (if (> _actual_use 0)
    (Components|Animation|PlayAnimation (Variables|Default|GetWeaponBody) "/Game/ArtMaterials/MilitaryWeapSilver/Weapons/Animations/Fire_Rifle_W.Fire_Rifle_W" false)
    (Camera|PlayWorldCameraShake "/Game/Blueprints/CamShake_01.CamShake_01_C" _returnvalue 0.0 5e+02 3.0)
    (bind (_outhit _returnvalue_3) (Collision|LineTraceByChannel (+ _returnvalue (* _returnvalue_2 6.0)) (+ _returnvalue (* _returnvalue_2 (Variables|Settings|GetShooting%20Range))) "TraceTypeQuery1" false 0 "None"))
    (if _returnvalue_3
      (Utilities|FlowControl|Sequence
        (:then_0
          (Utilities|Casting|CastToCharacter (.HitActor (Collision|BreakHitResult _outhit))
            (:then
              (Audio|PlaySoundatLocation "/Game/ArtMaterials/MilitaryWeapSilver/Sound/Rifle/Cues/Rifle_ImpactBody_Cue.Rifle_ImpactBody_Cue" (.Location (Collision|BreakHitResult _outhit)) "0, 0, 0" 1.0 1.0 0.0 0 0 0))
            (:CastFailed
              (Audio|PlaySoundatLocation "/Game/ArtMaterials/MilitaryWeapSilver/Sound/Rifle/Cues/Rifle_ImpactSurface_Cue.Rifle_ImpactSurface_Cue" (.Location (Collision|BreakHitResult _outhit)) "0, 0, 0" 1.0 1.0 0.0 0 0 0))))
        (:then_2
          (Effects|SpawnEmitteratLocation "/Game/Effects/P_Hit.P_Hit" (.Location (Collision|BreakHitResult _outhit)))
          (Game|Damage|ApplyDamage (.HitActor (Collision|BreakHitResult _outhit)) (Variables|Default|GetDamage%20Per%20Fire) (Pawn|GetController (Variables|Default|GetWeaponOwner)) self))))
    (else
      (Audio|PlaySoundatLocation "/Game/ArtMaterials/MilitaryWeapSilver/Sound/Rifle/Cues/Rifle_AmmoPickup_Cue.Rifle_AmmoPickup_Cue" (Transformation|GetWorldLocation (Variables|Default|GetWeaponBody)) "0, 0, 0" 1.0 1.0 0.0 0 0 0)
      (CallFunction|StopFire))))

(event EventOnDrop
  (|CallParentFunction))

(event EventOnPickup
  (params (Action%20Character :type Character%20Object%20Reference))
  (|CallParentFunction Action%20Character))

(fn ConstructionScript
  (|CallParentFunction))

(fn GetPickableInfo
  (return (Utilities|Struct|MakePickableItemDisplayData "/Game/Textures/Icons/controllerIconSprite_Sprite_3.controllerIconSprite_Sprite_3" "突击步枪" "使用5.56mm子弹" false 1)))