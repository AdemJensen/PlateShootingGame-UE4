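; AR-15 assault rifle weapon Blueprint, supplying cosmetics and pickup display data on top of its parent class.
; Construction fills the magazine; the fire event plays the weapon animation, or a sound when no shot fires.
; Hits spawn impact particles and sound chosen by a cast chain over physical material classes, with a particle-only fallback.
; Each hit also plays a world camera shake centred on the fire arrow.
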(event EventBeginPlay
  (|CallParentFunction))

(event Collision|EventActorBeginOverlap
  (params (OtherActor :type Actor%20Object%20Reference))
  (|CallParentFunction OtherActor))

(event EventTick
  (params (DeltaSeconds :type Float%20%28single-precision%29)))

(event EventMakeFireEffectBP
  (params (Fired :type Boolean))
  (if Fired
    (Components|Animation|PlayAnimation (Variables|Default|GetWeaponBody) "/Game/ArtMaterials/MilitaryWeapSilver/Weapons/Animations/Fire_Rifle_W.Fire_Rifle_W" false)
    (else
      (Audio|PlaySoundatLocation "/Game/ArtMaterials/MilitaryWeapSilver/Sound/Rifle/Cues/Rifle_AmmoPickup_Cue.Rifle_AmmoPickup_Cue" (Transformation|GetWorldLocation (Variables|Default|GetWeaponBody)) "0, 0, 0" 1.0 1.0 0.0 0 0 0))))

(event EventMakeHitEffectBP
  (params (HitPhysicalMaterial :type Physical%20Material%20Object%20Reference) (HitLocation :type Vector :default "0, 0, 0") (HitActor :type Actor%20Object%20Reference) (HitComponent :type Primitive%20Component%20Object%20Reference) (HitBoneName :type Name :default "None"))
  (bind (_partical_sys _sound_cue) (CallFunction|GetHitEffects HitPhysicalMaterial))
  (Audio|PlaySoundatLocation _sound_cue HitLocation "0, 0, 0" 1.0 1.0 0.0 0 0 0)
  (Effects|SpawnEmitteratLocation _partical_sys HitLocation)
  (Camera|PlayWorldCameraShake "/Game/Blueprints/CamShake_01.CamShake_01_C" (Transformation|GetWorldLocation (Variables|Default|GetWeaponFireArrow)) 0.0 5e+02 3.0))

(fn ConstructionScript
  (|CallParentFunction)
  (Variables|Default|SetMagRemain (Variables|Default|GetMagCapacity)))

(fn GetPickableInfo
  (return (Utilities|Struct|MakePickableItemDisplayData "/Game/Textures/Icons/controllerIconSprite_Sprite_3.controllerIconSprite_Sprite_3" "Testive Assault Rifle" "A Testive Assault rifle presented by C++." false 1)))

(fn GetHitEffects
  (params (Phys%20Mat :type Object%20Object%20Reference))
  (Utilities|FlowControl|Sequence
    (:then_0
      (Utilities|Casting|CastToMetal Phys%20Mat)
      (return "/Game/ArtMaterials/MilitaryWeapSilver/FX/P_Impact_Metal_Medium_01.P_Impact_Metal_Medium_01" "/Game/Audio/Bullet_Impact/BI_Metal_Heavy.BI_Metal_Heavy"))
    (:then_1
      (Utilities|Casting|CastToBrick Phys%20Mat)
      (return "/Game/ArtMaterials/MilitaryWeapSilver/FX/P_Impact_Stone_Medium_01.P_Impact_Stone_Medium_01" "/Game/Audio/Bullet_Impact/BI_Brick_Heavy.BI_Brick_Heavy"))
    (:then_2
      (Utilities|Casting|CastToDirt Phys%20Mat)
      (return "/Game/ArtMaterials/MilitaryWeapSilver/FX/P_Impact_Stone_Large_01.P_Impact_Stone_Large_01" "/Game/Audio/Bullet_Impact/BI_Dirt_Heavy.BI_Dirt_Heavy"))
    (:then_3
      (Utilities|Casting|CastToGlass Phys%20Mat)
      (return "/Game/Effects/P_Hit.P_Hit" "/Game/Audio/Bullet_Impact/BI_Glass_Heavy.BI_Glass_Heavy"))
    (:then_4
      (Utilities|Casting|CastToWood Phys%20Mat)
      (return "/Game/ArtMaterials/MilitaryWeapSilver/FX/P_Impact_Wood_Medium_01.P_Impact_Wood_Medium_01" "/Game/Audio/Bullet_Impact/BI_Wood_Heavy.BI_Wood_Heavy"))
    (:then_5
      (Utilities|Casting|CastToFlesh Phys%20Mat)
      (return "/Game/Effects/P_Hit_Blood.P_Hit_Blood" "/Game/ArtMaterials/Bullet_Impact_Sounds/Cues/bullet_impact_body_flesh_01_Cue.bullet_impact_body_flesh_01_Cue"))
    (:then_6
      (return "/Game/Effects/P_Hit.P_Hit" 0))))