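; Base weapon actor that characters can pick up, drop, fire and reload, with subclasses implementing the fire and reload hooks.
; Tick runs a server-only fire-rate accumulator that calls OnFire for single or continuous fire, while UseAmmo handles magazine consumption.
; A pickup-range overlap tracks I_HoldableCharacter actors and notifies them of availability.
; Pickup and drop set the owner, toggle body physics, update those characters and play sounds.
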(event OnComponentBeginOverlap(PickupRange)
  (params (OverlappedComponent :type Primitive%20Component%20Object%20Reference) (OtherActor :type Actor%20Object%20Reference) (OtherComp :type Primitive%20Component%20Object%20Reference) (OtherBodyIndex :type Integer) (bFromSweep :type Boolean) (SweepResult :type Hit%20Result%20Structure%20%28by%20ref%29))
  (if (Utilities|DoesObjectImplementInterface OtherActor "/Game/Blueprints/Weapons/I_HoldableCharacter.I_HoldableCharacter_C")
    (bind _asi_holdable_character (Utilities|Casting|CastToI_HoldableCharacter OtherActor))
    (Utilities|Array|AddUnique (Variables|Status|GetCharacters%20Waiting%20to%20me%20pickup) _asi_holdable_character)
    (if (not (Utilities|IsValid (Variables|设置|GetWeaponOwner)))
      (Default|OnAbletoPickItem _asi_holdable_character self))))

(event OnComponentEndOverlap(PickupRange)
  (params (OverlappedComponent :type Primitive%20Component%20Object%20Reference) (OtherActor :type Actor%20Object%20Reference) (OtherComp :type Primitive%20Component%20Object%20Reference) (OtherBodyIndex :type Integer))
  (if (Utilities|DoesObjectImplementInterface OtherActor "/Game/Blueprints/Weapons/I_HoldableCharacter.I_HoldableCharacter_C")
    (bind _asi_holdable_character (Utilities|Casting|CastToI_HoldableCharacter OtherActor))
    (bind _returnvalue (Utilities|Array|RemoveItem (Variables|Status|GetCharacters%20Waiting%20to%20me%20pickup) _asi_holdable_character))
    (if _returnvalue
      (Default|OnLostTrackonItem _asi_holdable_character self))))

(event Custom|Event%20On%20Drop%20Implementation
  (Variables|设置|SetWeaponOwner 0)
  (CallFunction|ClientSetSimulatePhysics true)
  (CallFunction|ClientAnnouncePlayers:AbletoPickup)
  (CallFunction|ClientPlayDropSounds))

(event Custom|Event%20On%20Pickup%20Implementation
  (params (Action%20Character :type Character%20Object%20Reference))
  (Variables|设置|SetWeaponOwner Action%20Character)
  (CallFunction|ClientSetSimulatePhysics false)
  (CallFunction|ClientAnnouncePlayers:LostTrack)
  (CallFunction|ClientPlayPickupSounds))

(event Custom|Action%20Reload
  (if (not (or (Variables|Status|GetIs%20Reloading) (not (Variables|设置|GetNeeds%20Reload))))
    (if (not (>= (Variables|Status|GetMag%20Remain) (Variables|设置|GetMag%20Capacity)))
      (Variables|Status|SetIs%20Reloading true)
      (Variables|Status|SetIs%20Firing false)
      (CallFunction|OnReloadStart))))

(event Custom|Action%20Stop%20Reload
  (params (Generate%20Interruption :type Boolean))
  (if (Variables|Status|GetIs%20Reloading)
    (Variables|Status|SetIs%20Reloading false)
    (CallFunction|OnReloadInterrupt)
    (if Generate%20Interruption
      (Default|CallOnReloadInterrupted))))

(event Custom|Client%20Play%20Drop%20Sounds
  (Audio|PlaySoundatLocation (Variables|设置|GetDrop%20Sound) (Transformation|GetWorldLocation (Variables|Default|GetWeaponBody)) "0, 0, 0" 1.0 1.0 0.0 0 0 0))

(event Custom|Client%20Set%20Simulate%20Physics
  (params (Simulate%20Physics :type Boolean))
  (bind _weaponbody (Variables|Default|GetWeaponBody))
  (Physics|SetSimulatePhysics _weaponbody Simulate%20Physics)
  (Physics|SetEnableGravity _weaponbody Simulate%20Physics))

(event Custom|Handle%20Fire
  (params (Delta%20Seconds :type Float%20%28single-precision%29))
  ;[1 1 1] Fire
  (if (Networking|IsServer)
    (if (< (Variables|Status|GetTime%20Since%20Last%20Fire) (* 2 (Variables|Settings|GetFire%20Rate)))
      (Variables|Status|SetTime%20Since%20Last%20Fire (+ Delta%20Seconds (Variables|Status|GetTime%20Since%20Last%20Fire))))
    (if (Variables|Status|GetIs%20Firing)
      (if (> (Variables|Status|GetTime%20Since%20Last%20Fire) (Variables|Settings|GetFire%20Rate))
        (Variables|Status|SetTime%20Since%20Last%20Fire (Math|Float|%(Float) (Variables|Status|GetTime%20Since%20Last%20Fire) (Variables|Settings|GetFire%20Rate)))
        (CallFunction|OnFire)
        (if (not (Variables|设置|GetFire%20Continuously))
          (CallFunction|ActionStopFire))))))

(event Custom|Client%20Play%20Pickup%20Sounds
  (Audio|PlaySoundatLocation (Variables|设置|GetPickup%20Sound) (Transformation|GetWorldLocation (Variables|Default|GetWeaponBody)) "0, 0, 0" 1.0 1.0 0.0 0 0 0))

(event Custom|Action%20Fire
  (Development|PrintString "Action FIre")
  (if (not (Variables|Status|GetIs%20Firing))
    (if (Variables|Status|GetIs%20Reloading)
      (if (not (<= (Variables|Status|GetMag%20Remain) 0))
        (CallFunction|ActionStopReload true)
        (Variables|Status|SetIs%20Firing true :!label _label))
      (else
        (goto _label)))))

(event Custom|Client%20Announce%20Players:%20Lost%20Track
  (for _array_element (Variables|Status|GetCharacters%20Waiting%20to%20me%20pickup)
    (Default|OnLostTrackonItem _array_element self))
  (Development|PrintText "On Pickup implementation"))

(event Custom|Action%20Stop%20Fire
  (Variables|Status|SetIs%20Firing false))

(event Custom|Client%20Announce%20Players:%20Able%20To%20Pickup
  (for _array_element (Variables|Status|GetCharacters%20Waiting%20to%20me%20pickup)
    (Default|OnAbletoPickItem _array_element self))
  (Development|PrintText "On Drop implementation"))

(event EventBeginPlay)

(event Collision|EventActorBeginOverlap
  (params (OtherActor :type Actor%20Object%20Reference)))

(event EventTick
  (params (DeltaSeconds :type Float%20%28single-precision%29))
  (CallFunction|HandleFire DeltaSeconds))

(event EventOnPickup
  (params (Action%20Character :type Character%20Object%20Reference))
  (CallFunction|EventonPickupImplementation Action%20Character))

(event EventOnDrop
  (CallFunction|EventonDropImplementation))

(event Custom|On%20Fire)

(event Custom|On%20Reload%20Interrupt)

(event Custom|On%20Reload%20Start)

(event Custom|On%20Reload%20Complete)

(fn ConstructionScript
  (Variables|Status|SetTime%20Since%20Last%20Fire (Variables|Settings|GetFire%20Rate))
  (Variables|Status|SetMag%20Remain (Variables|设置|GetMag%20Capacity))
  (Class|PrimitiveComponent|SetMassOverrideinKg (Variables|Default|GetWeaponBody) "None" (Variables|设置|GetMass%20in%20KG) true))

(fn GetWeaponFireLocation
  (return (Transformation|GetWorldLocation (Variables|Default|GetWeaponDirection))))

(fn GetWeaponTowardsRotation
  (return (Transformation|GetWorldRotation (Variables|Default|GetWeaponDirection))))

(fn SetFireRotation
  (params (Aiming%20Rotation :type Rotator))
  (Variables|设置|SetAiming%20Direction%20Vector (Math|Rotator|GetRotationXVector Aiming%20Rotation)))

(fn UseAmmo
  (params (Expected%20Ammo :type Integer) (Can%20use%20parcial :type Boolean))
  (if (Variables|设置|GetNeeds%20Reload)
    (if Can%20use%20parcial
      (if (>= (Variables|Status|GetMag%20Remain) Expected%20Ammo)
        _
        (else
          (LocalVariables|SetMag%20Use (Variables|Status|GetMag%20Remain))
          (Variables|Status|SetMag%20Remain 0)
          (return (LocalVariables|GetMag%20Use))))
      (elif (>= (Variables|Status|GetMag%20Remain) Expected%20Ammo)
        _
        (else
          (return 0))))
    (Variables|Status|SetMag%20Remain (- (Variables|Status|GetMag%20Remain) Expected%20Ammo))
    (return Expected%20Ammo)
    (else
      (return Expected%20Ammo))))

(fn GetHitSound
  (params (Phy%20Mat%20inst :type Physical%20Material%20Object%20Reference))
  (return 0))

(fn GetPickableInfo
  (return ""))

(fn IsOpenforPickup
  (return (Utilities|IsValid (Variables|设置|GetWeaponOwner))))