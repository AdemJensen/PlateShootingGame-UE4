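; Test ammo pickup actor that refills the magazine of a shooter character's weapon in hand to capacity.
; An overlap range tells HoldableActor implementers when they can pick it up or lose track of it.
; Pickup passes the acting character to a refill handler, then plays a rifle reload sound at the pickup mesh.
; It supplies display info, toggles an indicator widget, always reports open for pickup, and never removes itself.
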(event OnComponentBeginOverlap(OperationRange)
  (params (OverlappedComponent :type Primitive%20Component%20Object%20Reference) (OtherActor :type Actor%20Object%20Reference) (OtherComp :type Primitive%20Component%20Object%20Reference) (OtherBodyIndex :type Integer) (bFromSweep :type Boolean) (SweepResult :type Hit%20Result%20Structure%20%28by%20ref%29))
  (if (Utilities|DoesObjectImplementInterface OtherActor "/Script/PlateShootingGame.HoldableActor")
    (bind _asholdable_actor (Utilities|Casting|CastToHoldableActor OtherActor))
    (Class|HoldableActor|OnAbletoPickupItem _asholdable_actor self)))

(event OnComponentEndOverlap(OperationRange)
  (params (OverlappedComponent :type Primitive%20Component%20Object%20Reference) (OtherActor :type Actor%20Object%20Reference) (OtherComp :type Primitive%20Component%20Object%20Reference) (OtherBodyIndex :type Integer))
  (if (Utilities|DoesObjectImplementInterface OtherActor "/Script/PlateShootingGame.HoldableActor")
    (bind _asholdable_actor (Utilities|Casting|CastToHoldableActor OtherActor))
    (Class|HoldableActor|OnLostTrackOfItem _asholdable_actor self)))

(event Custom|Toggle%20Ammo%20indicator
  (params (Show :type Boolean))
  (Widget|SetVisibility (UserInterface|GetUserWidgetObject (Variables|Default|GetIndicator)) (select Show "Visible" "Collapsed")))

(event Custom|Handle%20Pickup
  (params (Action%20Character :type Character%20Object%20Reference))
  (bind _asshooter_game_character_base (Utilities|Casting|CastToShooterGameCharacterBase Action%20Character))
  (Variables|/Script/PlateShootingGame.Weapon|SetMagRemain (Variables|/Script/PlateShootingGame.ShooterGameCharacterBase|GetWeaponInHand _asshooter_game_character_base) (Variables|/Script/PlateShootingGame.Weapon|GetMagCapacity (Variables|/Script/PlateShootingGame.ShooterGameCharacterBase|GetWeaponInHand _asshooter_game_character_base)))
  (CallFunction|ClientPlaySound))

(event Custom|Client%20Play%20sound
  (Audio|PlaySoundatLocation "/Game/ArtMaterials/MilitaryWeapSilver/Sound/Rifle/Cues/Rifle_Reload_Cue.Rifle_Reload_Cue" (Transformation|GetWorldLocation (Variables|Default|GetAssaultRifle_Pickup)) "0, 0, 0" 1.0 1.0 0.0 0 0 0))

(event EventBeginPlay)

(event Collision|EventActorBeginOverlap
  (params (OtherActor :type Actor%20Object%20Reference)))

(event EventTick
  (params (DeltaSeconds :type Float%20%28single-precision%29)))

(event EventOnPickup
  (params (ActionActor :type Actor%20Object%20Reference))
  (bind _ascharacter (Utilities|Casting|CastToCharacter ActionActor))
  (CallFunction|HandlePickup _ascharacter))

(fn ConstructionScript)

(fn GetPickableInfo
  (return (Utilities|Struct|MakePickableItemDisplayData "/Game/Textures/Icons/controllerIconSprite_Sprite_5.controllerIconSprite_Sprite_5" "弹药" "各种弹药" false 1)))

(fn IsOpenforPickup
  (return true))