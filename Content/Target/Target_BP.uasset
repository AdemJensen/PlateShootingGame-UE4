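; A shootable target actor that shuttles back and forth, shows a health bar, and awards score to the instigator's player state when destroyed.
; Tick alternates timed move and halt phases, with only the server reversing velocity as each move begins.
; Initialize configures health, score, color and motion, using a flag to suppress bar updates during setup.
; RepNotify functions update the health bar widget and dynamic material color; death spawns a particle burst.
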(event Custom|Die
  (Effects|SpawnEmitteratLocation "/Game/Effects/P_MuzzleFlash.P_MuzzleFlash" (Transformation|GetWorldLocation (Variables|Default|GetMesh)) "0, 0, 0" "2.000000,2.000000,2.000000"))

(event EventBeginPlay
  (bind _ashealth_bar (Utilities|GetHealthBarObj)
    (:then
      (Default|Initialize _ashealth_bar 0.7 1.0 "(X=400.000000,Y=15.000000)"))))

(event Collision|EventActorBeginOverlap
  (params (OtherActor :type Actor%20Object%20Reference)))

(event EventTick
  (params (DeltaSeconds :type Float%20%28single-precision%29))
  (if (> (Math|Vector|VectorLength (Variables|movement|GetVelocity)) 0.0)
    (if (Variables|movement|GetIsMoving)
      (Transformation|SetActorLocation (+ (Transformation|GetActorLocation) (* (Variables|movement|GetVelocity) DeltaSeconds)) false false))
    (bind _output_get (Variables|Movement|SetNowSec (+ (Variables|Movement|GetNowSec) DeltaSeconds)))
    (if (> _output_get (Math|Float|SelectFloat (Variables|Movement|GetMoveTime) (Variables|Movement|GetHaltTime) (Variables|movement|GetIsMoving)))
      (Variables|movement|SetIsMoving (not (Variables|movement|GetIsMoving)))
      (Variables|Movement|SetNowSec 0.0)
      (if (and (Variables|movement|GetIsMoving) (Networking|IsServer))
        (Variables|movement|SetVelocity (* (Variables|movement|GetVelocity) -1))))))

(event Game|Damage|EventAnyDamage
  (params (Damage :type Float%20%28single-precision%29) (DamageType :type Damage%20Type%20Object%20Reference) (InstigatedBy :type Controller%20Object%20Reference) (DamageCauser :type Actor%20Object%20Reference))
  (Variables|Default|SetHealth (- (Variables|Default|GetHealth) (Math|Float|Floor Damage)))
  (if (<= (Variables|Default|GetHealth) 0)
    (bind _asmy_player_state (Utilities|Casting|CastToMyPlayerState (Variables|/Script/Engine.Controller|GetPlayerState InstigatedBy)))
    (Default|IncrementScore _asmy_player_state (Variables|Default|GetAddScore))
    (CallFunction|Die)
    (Actor|DestroyActor)))

(fn ConstructionScript
  (bind _returnvalue (Rendering|Material|CreateDynamicMaterialInstance (Variables|Default|GetMesh) 0 "/Game/Materials/M_Hat_Inst.M_Hat_Inst" "None" :!class /Script/Engine.PrimitiveComponent))
  (Variables|Default|SetMaterialInstance _returnvalue)
  (CallFunction|SetColor (Variables|Default|GetColor))
  (Variables|Default|SetMax_Health (Variables|Default|GetHealth)))

(fn SetColor
  (params (Color :type Linear%20Color%20Structure))
  (bind _output_get (Variables|Default|SetColor Color))
  (Rendering|Material|SetVectorParameterValue (Variables|Default|GetMaterialInstance) "Color" _output_get :!class /Script/Engine.MaterialInstanceDynamic))

(fn SetHealth
  (params (Health :type Integer))
  (bind _output_get (Variables|Default|SetHealth Health))
  (Variables|Default|SetMax_Health _output_get))

(fn Initialize
  (params (Health :type Integer) (AddScore :type Integer) (Color :type Linear%20Color%20Structure) (MoveTime :type Float%20%28single-precision%29) (HaltTime :type Float%20%28single-precision%29) (Velocity :type Vector))
  (Utilities|FlowControl|Sequence
    (:then_0
      (Variables|Default|SetOnInitState true))
    (:then_1
      (CallFunction|SetHealth Health))
    (:then_2
      (Variables|Default|SetAddScore AddScore))
    (:then_3
      (CallFunction|SetColor Color))
    (:then_4
      (Variables|Movement|SetMoveTime MoveTime))
    (:then_5
      (Variables|Movement|SetHaltTime HaltTime))
    (:then_6
      (Variables|movement|SetVelocity Velocity))
    (:then_7
      (Variables|Default|SetOnInitState false))))

(fn OnRepColor
  (Rendering|Material|SetVectorParameterValue (Variables|Default|GetMaterialInstance) "Color" (Variables|Default|GetColor) :!class /Script/Engine.MaterialInstanceDynamic))

(fn OnRepHealth
  (bind _ashealth_bar (Utilities|GetHealthBarObj)
    (:then
      (if (not (Variables|Default|GetOnInitState))
        (Default|SetNewValue _ashealth_bar (/ (Math|Conversions|ToFloat(Integer) (Variables|Default|GetHealth)) (Math|Conversions|ToFloat(Integer) (Variables|Default|GetMax_Health))))))))